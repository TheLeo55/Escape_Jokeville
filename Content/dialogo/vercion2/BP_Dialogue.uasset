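; BP_Dialogue is a trigger actor that opens a dialogue when an actor tagged "player" first overlaps its box.
; A DoOnce gates the overlap before the tag check, then a BW_Dialogue widget is created and added to the viewport.
; It deactivates the first-person character's movement, moves input from the character to itself, and shows the first DialogueTexts entry.
; The graph contains no logic to advance or close the dialogue.
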(event OnComponentBeginOverlap(Box)
  (params (OverlappedComponent :type Primitive%20Component%20Object%20Reference) (OtherActor :type Actor%20Object%20Reference) (OtherComp :type Primitive%20Component%20Object%20Reference) (OtherBodyIndex :type Integer) (bFromSweep :type Boolean) (SweepResult :type Hit%20Result%20Structure%20%28by%20ref%29))
  (bind _returnvalue (Game|GetPlayerController 0))
  (Utilities|FlowControl|DoOnce false
    (:Completed
      (if (Actor|ActorHasTag OtherActor "player")
        (bind _returnvalue_2 (UserInterface|CreateWidget "/Game/dialogo/vercion2/BW_Dialogue.BW_Dialogue_C"))
        (bind _output_get (Variables|Default|SetDialogueWidget _returnvalue_2))
        (UserInterface|Viewport|AddtoViewport (Variables|Default|GetDialogueWidget) 0)
        (Utilities|FlowControl|Sequence
          (:then_0
            (bind _asbp_first_person_character (Utilities|Casting|CastToBP_FirstPersonCharacter (Game|GetPlayerCharacter 0)))
            (Components|Activation|Deactivate (Variables|/Script/Engine.Character|GetCharacterMovement _asbp_first_person_character))
            (Input|DisableInput _asbp_first_person_character _returnvalue)
            (Input|EnableInput _returnvalue))
          (:then_1
            (Rendering|Components|TextRender|SetText (Variables|/Game/dialogo/vercion2/BW_Dialogue.BW_Dialogue_C|GetDialogueText (Variables|Default|GetDialogueWidget)) (Utilities|Array|Get(acopy) (Variables|Default|GetDialogueTexts)))))))))

(fn ConstructionScript)