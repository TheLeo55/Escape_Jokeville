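; BP_Colider is a dialogue trigger that shows a world-space text and a dialogue widget when the first-person character enters its box.
; Overlap begin unhides the TextRender and adds a new BW_Ele widget to the viewport; overlap end reverses both.
; EventDiagol passes the Text lines to the widget, reveals its background and text, and advances the row, removing the widget after the last.
; A DoOnce gates each step and resets immediately afterwards.
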(event OnComponentBeginOverlap(Box)
  (params (OverlappedComponent :type Primitive%20Component%20Object%20Reference) (OtherActor :type Actor%20Object%20Reference) (OtherComp :type Primitive%20Component%20Object%20Reference) (OtherBodyIndex :type Integer) (bFromSweep :type Boolean) (SweepResult :type Hit%20Result%20Structure%20%28by%20ref%29))
  (Utilities|Casting|CastToBP_FirstPersonCharacter OtherActor)
  (Development|SetHiddeninGame (Variables|Default|GetTextRender) false false)
  (bind _returnvalue (UserInterface|CreateWidget "/Game/dialogo/BW_Ele.BW_Ele_C"))
  (bind _output_get (Variables|Default|SetDialog%20UI _returnvalue))
  (UserInterface|Viewport|AddtoViewport _output_get 0))

(event OnComponentEndOverlap(Box)
  (params (OverlappedComponent :type Primitive%20Component%20Object%20Reference) (OtherActor :type Actor%20Object%20Reference) (OtherComp :type Primitive%20Component%20Object%20Reference) (OtherBodyIndex :type Integer))
  (bind _dialog_ui (Variables|Default|GetDialog%20UI))
  (Utilities|Casting|CastToBP_FirstPersonCharacter OtherActor)
  (Development|SetHiddeninGame (Variables|Default|GetTextRender) true false)
  (Utilities|IsValid _dialog_ui
    (:Is%20Valid
      (Widget|RemovefromParent _dialog_ui))))

(event Custom|ResetDoOnce
  (bind _dialog_ui (Variables|Default|GetDialog%20UI))
  (bind _dialog_ui_2 (Variables|Default|GetDialog%20UI))
  (Utilities|FlowControl|DoOnce false) ; enters at Reset
)

(event EventEventDiagol
  (bind _dialog_ui (Variables|Default|GetDialog%20UI))
  (bind _dialog_ui_2 (Variables|Default|GetDialog%20UI))
  (Utilities|FlowControl|DoOnce false
    (:Completed
      (Variables|/Game/dialogo/BW_Ele.BW_Ele_C|SetText _dialog_ui_2 (Variables|Default|GetText))
      (Widget|SetVisibility (Variables|/Game/dialogo/BW_Ele.BW_Ele_C|Getfondo _dialog_ui_2) "Visible")
      (if (> (+ (Variables|/Game/dialogo/BW_Ele.BW_Ele_C|GetTextRow (Variables|Default|GetDialog%20UI)) 1) (- (Utilities|Array|Length (Variables|Default|GetText)) 1))
        (Widget|RemovefromParent _dialog_ui)
        (CallFunction|ResetDoOnce)
        (else
          (Variables|/Game/dialogo/BW_Ele.BW_Ele_C|SetTextRow _dialog_ui (+ (Variables|/Game/dialogo/BW_Ele.BW_Ele_C|GetTextRow (Variables|Default|GetDialog%20UI)) 1))
          (CallFunction|ResetDoOnce))))))

(fn ConstructionScript)