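; BP_NPC is an NPC that shows a one-time dialogue when its Box is first overlapped.
; The overlap creates a Dialogo widget, freezes the first-person player's movement and input, and takes input itself; it does not filter the overlapping actor.
; IA_Action steps through the DialogueText array.
; Past the last line, it returns input, plays the StartDialogue animation in reverse and reactivates movement after a short delay.
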(event OnComponentBeginOverlap(Box)
  (params (OverlappedComponent :type Primitive%20Component%20Object%20Reference) (OtherActor :type Actor%20Object%20Reference) (OtherComp :type Primitive%20Component%20Object%20Reference) (OtherBodyIndex :type Integer) (bFromSweep :type Boolean) (SweepResult :type Hit%20Result%20Structure%20%28by%20ref%29))
  (bind _returnvalue (Game|GetPlayerController 0))
  (Utilities|FlowControl|DoOnce false
    (:Completed
      (if true
        (Development|PrintText "Si aceptó el tipo de actor")
        (bind _returnvalue_2 (UserInterface|CreateWidget "/Game/Dialogos/Dialogo.Dialogo_C"))
        (bind _output_get (Variables|Default|SetDialogue%20Widget _returnvalue_2))
        (UserInterface|Viewport|AddtoViewport _output_get 0)
        (Utilities|FlowControl|Sequence
          (:then_0
            (bind _asbp_first_person_character (Utilities|Casting|CastToBP_FirstPersonCharacter (Game|GetPlayerCharacter 0)))
            (Components|Activation|Deactivate (Variables|/Script/Engine.Character|GetCharacterMovement _asbp_first_person_character))
            (Input|DisableInput _asbp_first_person_character _returnvalue)
            (Input|EnableInput _returnvalue))
          (:then_1
            (Rendering|Components|TextRender|SetText (Variables|/Game/Dialogos/Dialogo.Dialogo_C|GetDialogueText (Variables|Default|GetDialogue%20Widget)) (Utilities|Array|Get(acopy) (Variables|Default|GetDialogueText)))))))))

(event Input|EnhancedActionEvents|EnhancedInputActionIA_Action
  (params (ActionValue :type Boolean) (ElapsedSeconds :type Float%20%28double-precision%29) (TriggeredSeconds :type Float%20%28double-precision%29) (InputAction :type Input%20Action%20Object%20Reference :default "/Game/FirstPerson/Input/Actions/IA_Action.IA_Action"))
  (bind _returnvalue (Game|GetPlayerController 0))
  (bind _dialogue_widget (Variables|Default|GetDialogue%20Widget))
  (bind _index (Variables|Default|GetIndex))
  (:Started
    (Math|Integer|IncrementInt _index
      (:%20%20
        (if (<= _index (Utilities|Array|LastIndex (Variables|Default|GetDialogueText)))
          (Rendering|Components|TextRender|SetText (Variables|/Game/Dialogos/Dialogo.Dialogo_C|GetDialogueText (Variables|Default|GetDialogue%20Widget)) (Utilities|Array|Get(acopy) (Variables|Default|GetDialogueText) (Variables|Default|GetIndex)))
          (else
            (bind _asbp_first_person_character (Utilities|Casting|CastToBP_FirstPersonCharacter (Game|GetPlayerCharacter 0)))
            (Input|DisableInput _returnvalue)
            (Input|EnableInput _asbp_first_person_character _returnvalue)
            (Class|UserWidget|PlayAnimationReverse _dialogue_widget (Variables|/Game/Dialogos/Dialogo.Dialogo_C|GetStartDialogue _dialogue_widget) 1.0 false)
            (Utilities|FlowControl|Delay 1.0)
            (Components|Activation|Activate (Variables|/Script/Engine.Character|GetCharacterMovement _asbp_first_person_character) false)))))))

(fn ConstructionScript)